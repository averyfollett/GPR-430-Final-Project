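; BP_PlayerCharacter is a player character Blueprint whose only logic turns the character to face a Generator actor.
; The RotatetoGenerator event plays a timeline from the start, blending yaw toward the look-at rotation by its LerpFactor while keeping pitch and roll.
; Each update blends from the current yaw instead of a cached start, using a plain float Lerp with no angle wrapping.
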(event `self.RotateToGenerator`
  (bind (_direction _lerpfactor) (`Timeline|Timeline_0` :!via `PlayFromStart`)
    (:`Update`
      (`self.K2_SetActorRotation` (`KismetMathLibrary.MakeRotator` (.roll (`self.K2_GetActorRotation`)) (.pitch (`self.K2_GetActorRotation`)) (`KismetMathLibrary.Lerp` (.yaw (`self.K2_GetActorRotation`)) (.yaw (`KismetMathLibrary.FindLookAtRotation` (`self.K2_GetActorLocation`) (`self.K2_GetActorLocation` (`self.Generator`)))) _lerpfactor))))))

(fn `UserConstructionScript`)