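; BP_SlidingDoor is a sliding door with left and right panels, each paired with an inverted counterpart.
; MoveLeftDoor and MoveRightDoor events each play their own timeline independently.
; Each timeline's Driver track lerps that side's two meshes between stored start and end relative locations.
; The graph only plays the timelines forward and holds no trigger or closing logic.
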(event `self.MoveLeftDoor`
  (bind (_direction _driver) (`Timeline|Timeline_0`)
    (:`Update`
      (`SceneComponent.K2_SetRelativeLocation` (`self.LeftDoor`) (`KismetMathLibrary.VLerp` (`self.LeftDoorStart`) (`self.LeftDoorEnd`) _driver) false false)
      (`SceneComponent.K2_SetRelativeLocation` (`self.LeftDoorInverted`) (`KismetMathLibrary.VLerp` (`self.LeftDoorInvertedStart`) (`self.LeftDoorInvertedEnd`) _driver) false false))))

(event `self.MoveRightDoor`
  (bind (_direction _driver) (`Timeline|Timeline_1`)
    (:`Update`
      (`SceneComponent.K2_SetRelativeLocation` (`self.RightDoor`) (`KismetMathLibrary.VLerp` (`self.RightDoorStart`) (`self.RightDoorEnd`) _driver) false false)
      (`SceneComponent.K2_SetRelativeLocation` (`self.RightDoorInverted`) (`KismetMathLibrary.VLerp` (`self.RightDoorInvertedStart`) (`self.RightDoorInvertedEnd`) _driver) false false))))

(fn `UserConstructionScript`)