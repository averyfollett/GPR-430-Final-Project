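; BP_SplineWire is a wire actor that builds its shape along an editable spline in the construction script.
; For each pair of neighboring points on SplineWireComponent, it adds a Z-forward spline mesh attached to the spline and stores it in SplineMeshes.
; Each segment takes its local start and end positions and tangents from those points, so the wire bends with the curve.
; The event graph has no active logic.
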(fn `UserConstructionScript`
  (for _index (range (+ (- (`SplineComponent.GetNumberOfSplinePoints` (`self.SplineWireComponent`)) 2) 1))
    (bind _returnvalue (`AddComponent|NODE_AddSplineMeshComponent-0`))
    (`KismetArrayLibrary.Array_Add` (`self.SplineMeshes`) _returnvalue)
    (`SplineMeshComponent.SetForwardAxis` _returnvalue "Z" true)
    (`self.K2_AttachToComponent` (`self.SplineWireComponent`) "None" "KeepRelative" "KeepRelative" "KeepRelative")
    (bind (_location _tangent) (`SplineComponent.GetLocationAndTangentAtSplinePoint` (`self.SplineWireComponent`) _index "Local"))
    (bind (_location_2 _tangent_2) (`SplineComponent.GetLocationAndTangentAtSplinePoint` (`self.SplineWireComponent`) (+ _index 1) "Local"))
    (`SplineMeshComponent.SetStartAndEnd` _returnvalue _location _tangent _location_2 _tangent_2 true)))