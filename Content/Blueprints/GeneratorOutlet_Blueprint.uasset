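; Generator outlet actor that powers a list of linked objects when a generator is placed in it.
; Overlapping a generator that is not held snaps it above the outlet with sparks, while a timeline rotates it, turns the emissive material green and powers the objects.
; Power messages carry a per-outlet GUID as setter ID.
; GeneratorPickedUp cuts power without changing color; the end-overlap shutoff logic is disconnected.
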(event `self.ReceiveBeginPlay`
  ;[0 1 0.07355] Completed
  ;;[1 1 1] Create new GUID
  (set `self.ThisGuid` (`KismetGuidLibrary.NewGuid`))
  ;;[1 1 1] Create Dynamic Material
  (bind _returnvalue (`PrimitiveComponent.CreateDynamicMaterialInstance` (`self.Cube`) 0 null "None"))
  (set `self.generatorOutletMaterial` _returnvalue))

(event `Set List Power State`
  (params (isPowered :type Boolean))
  ;[0 1 0.07355] Completed
  ;;[1 1 1] Set the power state of all connections
  (for _array_element (`self.PoweredObjects`)
    (message `/Game/Blueprints/WireElements/Powerable.Set Powered` _array_element isPowered (`self.ThisGuid`))))

(event `Snap to center`
  (params (Generator :type "/Game/Blueprints/Generator_Blueprint_New Object Reference"))
  (bind _returnvalue (+ (`self.K2_GetActorLocation`) (0.0 7.0 10.0)))
  ;[0 1 0.07355] Completed
  ;;[1 1 1] Snap to center
  (`self.K2_SetActorLocation` Generator _returnvalue false false)
  (`GameplayStatics.SpawnEmitterAtLocation` (`self.sparksParticles`) _returnvalue)
  (bind (_direction _zrotation) (`Timeline|rotateGenerator` :!via `PlayFromStart`)
    (:`Update`
      (`self.K2_SetActorRotation` Generator (`KismetMathLibrary.MakeRotator` 0.0 0.0 _zrotation) false)
      (`self.Change To Green`)
      (`self.Set List Power State` true))))

(event `Generator Picked Up`
  ;[0 1 0.07355] Completed
  ;;[1 1 1] Generator Picked up
  (`self.Set List Power State` false))

(event `Change To Green`
  ;[0 1 0.07355] Completed
  ;;[1 1 1] Change Colors
  (`MaterialInstanceDynamic.SetVectorParameterValue` (`self.generatorOutletMaterial`) "Emissive Color" (`KismetMathLibrary.MakeColor` 0.0 1.0)))

(event `Change To Red`
  ;[0 1 0.07355] Completed
  ;;[1 1 1] Change Colors
  (`MaterialInstanceDynamic.SetVectorParameterValue` (`self.generatorOutletMaterial`) "Emissive Color" (`KismetMathLibrary.MakeColor` 1.0)))

(event `self.ReceiveActorBeginOverlap`
  (params (OtherActor :type "Actor Object Reference"))
  ;[0 1 0.07355] Completed
  ;;[1 1 1] Generator Placed
  (`KismetSystemLibrary.PrintString` "OVERLAP DETECTED")
  (if (== (`GameplayStatics.GetObjectClass` OtherActor) "/Game/Blueprints/Generator_Blueprint_New.Generator_Blueprint_New_C")
    (set `self.IsPressed` true)
    (bind _asgenerator_blueprint_new (cast `/Game/Blueprints/Generator_Blueprint_New` OtherActor))
    (if (not (`/Game/Blueprints/Generator_Blueprint_New.isHeld` _asgenerator_blueprint_new))
      (`self.Snap to center` _asgenerator_blueprint_new) ; Also sets the next power state. IDK why, but you have to set it inside this function or it does not work
    )))

(event `self.ReceiveActorEndOverlap`
  (params (OtherActor :type "Actor Object Reference"))
  ;[0 1 0.07355] Completed
  ;;[1 1 1] Generator Removed
)

(fn `UserConstructionScript`)