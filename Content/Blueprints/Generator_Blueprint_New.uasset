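; Generator Blueprint is a carryable generator that tracks who holds it and interacts with generator outlets.
; When a new holder is set, it notifies a valid, different previous holder that the generator was stolen, then stores the new one.
; On pickup or release, it checks overlapping actors for outlets, signaling them on pickup or asking them to snap it to center on release.
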(event `Set held by`
  (params (newOwner :type "/Game/Blueprints/ThirdPersonBP/Blueprints/ThirdPersonCharacter Object Reference"))
  (bind _healdby (`self.HealdBy`))
  ;[0.1514 1 0] Completed
  ;;[1 1 1] Set held by
  (if (and (`KismetSystemLibrary.IsValid` _healdby) (`KismetSystemLibrary.IsValid` newOwner))
    (`KismetSystemLibrary.PrintString` "Old owner was valid")
    (if (!= newOwner _healdby)
      (`KismetSystemLibrary.PrintString` "Old owner not self")
      (`/Game/Blueprints/ThirdPersonBP/Blueprints/ThirdPersonCharacter.Generator Stolen` _healdby))
    (else
      (`KismetSystemLibrary.PrintString` "Old owner was nothing")))
  (set `self.HealdBy` newOwner))

(event `Being Picked Up Or Released`
  (params (isPickedUp :type Boolean))
  ;[0.1514 1 0] Completed
  ;;[1 1 1] Trigger outlet locking or unlocking
  (for _array_element (`self.GetOverlappingActors` null)
    (bind _asgenerator_outlet_blueprint (cast `/Game/Blueprints/GeneratorOutlet_Blueprint` _array_element))
    (if isPickedUp
      (`/Game/Blueprints/GeneratorOutlet_Blueprint.Generator Picked Up` _asgenerator_outlet_blueprint)
      (else
        (`/Game/Blueprints/GeneratorOutlet_Blueprint.Snap to center` _asgenerator_outlet_blueprint self)))))

(fn `UserConstructionScript`)