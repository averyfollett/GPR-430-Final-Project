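; PanCamera is a camera actor that takes over player 0's view and glides toward a target location.
; BeginPlay seeds the target location and rotation from its own transform, and Tick reasserts the view target every frame.
; Tick lerps location by Speed until within tolerance; rotation interpolation is unwired, leaving NewRotation unset in the move call.
; A note marks the work as finished in C++.
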(event `self.ReceiveBeginPlay`
  ;[0.01954 1 0] Finished in C++
  ;;[1 1 1] Set default camera location
  (`PlayerController.SetViewTargetWithBlend` (`GameplayStatics.GetPlayerController` 0) self 0.0 "VTBlend_Linear" 0.0 false)
  (set `self.TargetLocation` (`self.K2_GetActorLocation`))
  (set `self.TargetRotation` (`self.K2_GetActorRotation`)))

(event `self.ReceiveTick`
  (params (DeltaSeconds :type "Float (single-precision)"))
  (bind _returnvalue (`self.K2_GetActorLocation`))
  (bind _targetlocation (`self.TargetLocation`))
  ;[0.01954 1 0] Finished in C++
  ;;[1 1 1] move camera to new target location
  (`PlayerController.SetViewTargetWithBlend` (`GameplayStatics.GetPlayerController` 0) self 0.0 "VTBlend_Linear" 0.0 false)
  (if (not (== _targetlocation _returnvalue :`ErrorTolerance` 0.1))
    (`self.K2_SetActorLocationAndRotation` (`KismetMathLibrary.VLerp` _returnvalue _targetlocation (`self.Speed`)))))

(fn `UserConstructionScript`)