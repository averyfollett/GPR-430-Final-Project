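; Powerable turret that, while powered, launches any Character entering its ViewArea away from itself, using a scaled direction plus an added launch modifier.
; SetPowered stores the state, switches base and head emissive between green and red through dynamic materials, and toggles the PSPSHHH effect.
; Powering on also calls Sound, which uses DoOnce gates and random delays around turning playback.
; BeginPlay creates the materials and a GUID, exposed through GetGUID.
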(event `Set Apperance`
  (params (isPowered :type Boolean))
  (bind _returnvalue (`KismetMathLibrary.MakeColor` 1.0))
  (bind _returnvalue_2 (`KismetMathLibrary.MakeColor` 0.0 1.0))
  (bind _turretbasematerial (`self.turretBaseMaterial`))
  ;[1 1 1] Set apperance
  (if isPowered
    ;;[1 1 1] Change Color to Green
    (`MaterialInstanceDynamic.SetVectorParameterValue` (`self.turretBaseMaterial`) "Emissive Color" _returnvalue_2)
    (`MaterialInstanceDynamic.SetVectorParameterValue` (`self.turretHeadMaterial`) "Emissive Color" _returnvalue_2)
    (`ActorComponent.Activate` (`self.PS_PSHHH`) false)
    (else
      ;;[1 1 1] Change Color to Red (errors should be fixed)
      (`/Engine/EditorBlueprintResources/StandardMacros.IsValid` _turretbasematerial
        (:`Is Valid`
          (`MaterialInstanceDynamic.SetVectorParameterValue` _turretbasematerial "Emissive Color" _returnvalue)
          (`MaterialInstanceDynamic.SetVectorParameterValue` (`self.turretHeadMaterial`) "Emissive Color" _returnvalue)
          (`ActorComponent.Deactivate` (`self.PS_PSHHH`)))))))

(event `/Game/Blueprints/WireElements/Powerable.Set Powered`
  (params (isPowered :type Boolean) (setterID :type "Guid Structure"))
  ;[1 1 1] Set powered
  (set `self.Powered` isPowered)
  (`self.Set Apperance` isPowered)
  (if isPowered
    (`/Engine/EditorBlueprintResources/StandardMacros.DoOnce` false :!label _label
      (:`Completed`
        (`self.PlayTurning` false
          (:`End`
            (`/Engine/EditorBlueprintResources/StandardMacros.DoOnce` false :!via `Reset`
              (:`Completed`
                (`self.PlayTurning` true :!via `Stop`
                  (:`End`
                    (goto _label :!via `Reset`)))))))))))

(event `Launch Player`
  (params (targetActor :type "Actor Object Reference"))
  ;[1 1 1] Launch Target
  (if (`self.Powered`)
    (bind _ascharacter (cast `Character` targetActor))
    (`Character.LaunchCharacter` _ascharacter (+ (* (`KismetMathLibrary.Normal` (- (`self.K2_GetActorLocation` targetActor) (`self.K2_GetActorLocation`))) (`self.Strength`)) (`self.launchModifier`)) true true)
    (`/Engine/EditorBlueprintResources/StandardMacros.DoOnce` false :!label _label_2)
    (else
      (goto _label_2 :!via `Reset`))))

(event `self.ReceiveBeginPlay`
  ;[1 1 1] Beginning Set up
  ;[1 1 1] Create Dynamic Materials
  (bind _returnvalue (`PrimitiveComponent.CreateDynamicMaterialInstance` (`self.Base`) 0 null "None"))
  (set `self.turretBaseMaterial` _returnvalue)
  (bind _returnvalue_2 (`PrimitiveComponent.CreateDynamicMaterialInstance` (`self.SM_turretTop_01`) 0 null "None"))
  (set `self.turretHeadMaterial` _returnvalue_2)
  (set `self.thisGuid` (`KismetGuidLibrary.NewGuid`))
  (if (`self.Powered`)
    _))

(event `self.ViewArea.OnComponentBeginOverlap`
  (params (OverlappedComponent :type "PrimitiveComponent Object Reference") (OtherActor :type "Actor Object Reference") (OtherComp :type "PrimitiveComponent Object Reference") (OtherBodyIndex :type Integer) (bFromSweep :type Boolean) (SweepResult :type "HitResult Structure (by ref)"))
  ;[1 1 1] on overlap trigger
  (`self.Launch Player` OtherActor))

(fn `Get GUID`
  (returns (GUID :type "Guid Structure"))
  (return (`self.thisGuid`)))

(fn `UserConstructionScript`)