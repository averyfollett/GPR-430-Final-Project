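; Rotatable wire junction that passes power from the input selected by its current angle to that input's paired output.
; BeginPlay maps input GUIDs to outputs and creates a dynamic material that shows the powered state.
; Every input's last reported state is cached, but only the current source drives appearance and output.
; Rotating cuts the old output, steps to the next angle and applies the new source's cached state.
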(event `Set Next Powered`
  (params (isPowered :type Boolean) (powerSource :type "Guid Structure"))
  ;[0.05148 1 0] Completed in C++
  ;;[1 1 1] Set Next Powered
  (message `/Game/Blueprints/WireElements/Powerable.Set Powered` (`BlueprintMapLibrary.Map_Find` (`self.InputIdToOutput`) powerSource) isPowered (`self.thisGuid`)))

(event `Set Apperance`
  (params (isPowered :type Boolean))
  (bind _dynamic_material_instance (`self.Dynamic Material Instance`))
  ;[0.05148 1 0] Completed in C++
  ;;[1 1 1] Set Apperance
  (`MaterialInstanceDynamic.SetScalarParameterValue` _dynamic_material_instance "On/Off" (`KismetMathLibrary.Conv_BoolToDouble` isPowered))
  (`PrimitiveComponent.SetMaterial` (`self.Cylinder1`) 0 _dynamic_material_instance))

(event `Set stuff powered`
  (params (isPowered :type Boolean) (setterID :type "Guid Structure"))
  ;[0.05148 1 0] Completed in C++
  ;;[1 1 1] Set Powered
  (`BlueprintMapLibrary.Map_Add` (`self.LastReportedPowerState`) setterID isPowered) ; Store the reported power state of any input even if it is not the current one so that it can be used later when interface rotates
  (if (== setterID (`self.currentPowerSource`))
    (`self.Set Apperance` isPowered)
    (`self.Set Next Powered` isPowered setterID)))

(event `self.Set Powered`
  (params (isPowered :type Boolean) (setterID :type "Guid Structure"))
  ;[0.05148 1 0] Completed in C++
  ;;[1 1 1] Set Powered
  (`self.Set stuff powered` isPowered setterID))

(event `self.ReceiveBeginPlay`
  ;[0.05148 1 0] Completed in C++
  ;;[1 1 1] Inital Set Up
  (set `self.StartingRotation` (`self.K2_GetActorRotation`))
  (set `self.thisGuid` (`KismetGuidLibrary.NewGuid`))
  (bind _returnvalue (`PrimitiveComponent.CreateDynamicMaterialInstance` (`self.Cylinder1`) 0 null "None"))
  (set `self.Dynamic Material Instance` _returnvalue)
  (bind _keys (`BlueprintMapLibrary.Map_Keys` (`self.InputsAndOutputs`)))
  (for _array_element _keys
    (bind _guid (message `/Game/Blueprints/WireElements/Powerable.Get GUID` _array_element))
    (`BlueprintMapLibrary.Map_Add` (`self.InputIdToOutput`) _guid (`BlueprintMapLibrary.Map_Find` (`self.InputsAndOutputs`) _array_element)))
  (bind _guid_2 (message `/Game/Blueprints/WireElements/Powerable.Get GUID` (`self.firstPowerSource`)))
  (set `self.currentPowerSource` _guid_2)
  (bind _keys_2 (`BlueprintMapLibrary.Map_Keys` (`self.AnglesToInputs`)))
  (set `self.AngleList` _keys_2))

(event `/Game/Blueprints/WireElements/WireInterface.RotateWire`
  (bind _output (`|GetArrayItem` (`self.AngleList`) (`self.currentAngleIndex`)))
  ;[0.05148 1 0] Completed in C++
  ;;[1 1 1] Rotate
  (`self.Set Next Powered` false (`self.currentPowerSource`)) ; Remove power from currently powered output
  (set `self.currentAngleIndex` (mod (+ (`self.currentAngleIndex`) 1) (`KismetArrayLibrary.Array_Length` (`self.AngleList`))))
  (`self.K2_SetActorRotation` (`KismetMathLibrary.MakeRotator` 0.0 0.0 (+ (.yaw (`self.StartingRotation`)) _output)))
  (bind _guid (message `/Game/Blueprints/WireElements/Powerable.Get GUID` (`BlueprintMapLibrary.Map_Find` (`self.AnglesToInputs`) _output)))
  (bind _output_get (set `self.currentPowerSource` _guid))
  (`self.Set Powered` (`BlueprintMapLibrary.Map_Find` (`self.LastReportedPowerState`) _output_get) _output_get))

(fn `Get GUID`
  (returns (GUID :type "Guid Structure"))
  (return (`self.thisGuid`)))

(fn `UserConstructionScript`)